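; Shield Blueprint that plays a small looping vertical bob on its Shield component using keyframes coded in the graph.
; Tick accumulates time, advances a wrapping frame counter each FrameRate interval, and maps specific frames to target Z offsets.
; On the other ticks, it eases the component's relative location toward that target with a clamped delta-time lerp, keeping rotation and scale unchanged.
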(event `self.ReceiveTick`
  (params (DeltaSeconds :type "Float (single-precision)"))
  (bind _shield (`self.shield`))
  (bind _returnvalue (+ (`self.Frame`) 1))
  ;[1 1 1] Set Up Frame Rate
  (bind _output_get (set `self.TimeSinceFrame` (+ DeltaSeconds (`self.TimeSinceFrame`))))
  (if (< _output_get (`self.FrameRate`))
    ;[1 1 1] Animate
    (`SceneComponent.K2_SetRelativeTransform` _shield (`KismetMathLibrary.MakeTransform` (`KismetMathLibrary.VLerp` (.location (`SceneComponent.GetRelativeTransform` _shield)) (`self.TargetPos`) (`KismetMathLibrary.FClamp` (* DeltaSeconds (`self.LerpSpeed`)))) (.rotation (`SceneComponent.GetRelativeTransform` _shield)) (.scale (`SceneComponent.GetRelativeTransform` _shield))) false false)
    (else
      ;[1 1 1] Frame Decoder
      (set `self.TimeSinceFrame` 0.0)
      (if (> _returnvalue (- (`self.MaxFrames`) 1))
        (set `self.Frame` 0)
        (else
          (set `self.Frame` _returnvalue)))
      ;[1 1 1] Animation Keyframes
      (switch `int` (`self.Frame`)
        (:`0`
          (set `self.TargetPos` (0.0 0.0 0.0)))
        (:`1`
          (set `self.TargetPos` (0.0 0.0 -2.0)))
        (:`2`
          (set `self.TargetPos` (0.0 0.0 -5.0)))
        (:`4`
          (set `self.TargetPos` (0.0 0.0 0.0)))))))

(fn `UserConstructionScript`)