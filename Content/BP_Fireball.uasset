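; BP_Fireball is a physics-driven fireball actor that launches itself and carries a fire effect.
; One second after BeginPlay, it applies a mass-independent impulse scaled from LaunchForce to the Fireball component.
; Tick moves NSFire to the physics object's world location, since the effect follows the simulated body, and accumulates elapsed time.
; A Chaos collision deactivates the fire only after the first second, ignoring earlier contacts.
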(event `self.Fireball.OnChaosPhysicsCollision`
  (params (CollisionInfo :type "ChaosPhysicsCollisionInfo Structure (by ref)"))
  ;[1 1 1] Put Fire Out
  (if (> (`self.TimeElapsed`) 1.0)
    (`ActorComponent.Deactivate` (`self.NS_Fire`))))

(event `self.ReceiveTick`
  (params (DeltaSeconds :type "Float (single-precision)"))
  ;[1 1 1] Update Fire Location Due To Physics Object
  (set `self.TimeElapsed` (+ DeltaSeconds (`self.TimeElapsed`)))
  (`SceneComponent.K2_SetWorldLocation` (`self.NS_Fire`) (.location (`PhysicsObjectBlueprintLibrary.GetPhysicsObjectWorldTransform` (`self.Fireball`))) false false))

(event `self.ReceiveBeginPlay`
  ;[1 1 1] Launch Fireball
  (`KismetSystemLibrary.Delay` 1.0)
  (`PrimitiveComponent.AddImpulse` (`self.Fireball`) (* (`self.Launch Force`) (`KismetMathLibrary.Conv_IntToVector` 1000)) "None" true))

(fn `UserConstructionScript`)