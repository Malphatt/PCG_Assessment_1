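; BP_BreakableWall is a Chaos geometry collection wall that reacts to physics collisions.
; Tick advances two timers, ignoring collisions in the first second and separating isolated hits from rapid follow-ups.
; A collision over a second after the last spawns scaled smoke at EmissionPoint, later deactivated and destroyed after delays.
; Collisions in quicker succession instead set CeaseFire on every BP_SpawnFireball actor, and both cases reset the collision timer.
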(event `Spawn Smoke`
  ;[1 1 1] On Wall Collision
  (bind _returnvalue (`GameplayStatics.SpawnEmitterAtLocation` "/Game/StarterContent/Particles/P_Smoke.P_Smoke" (`SceneComponent.K2_GetComponentLocation` (`self.Emission Point`)) (struct) (10.0 10.0 10.0)))
  (`KismetSystemLibrary.Delay` 2.0)
  (`ActorComponent.Deactivate` _returnvalue)
  (`KismetSystemLibrary.Delay` 5.0)
  (`ActorComponent.K2_DestroyComponent` _returnvalue))

(event `self.GC_sop_Malphatt_breakablewall_1_0.OnChaosPhysicsCollision`
  (params (CollisionInfo :type "ChaosPhysicsCollisionInfo Structure (by ref)"))
  (bind _returnvalue (> (`self.TimeElapsed`) 1.0))
  ;[1 1 1] On Collision
  (if (and _returnvalue (> (`self.TimeSinceLastCollision`) 1.0))
    (set `self.TimeSinceLastCollision` 0.0)
    (`self.Spawn Smoke`)
    (elif _returnvalue
      (set `self.TimeSinceLastCollision` 0.0)
      (bind _outactors (`GameplayStatics.GetAllActorsOfClass` "/Game/BP_SpawnFireball.BP_SpawnFireball_C"))
      (for _array_element _outactors
        (set `/Game/BP_SpawnFireball.CeaseFire` true _array_element)))))

(event `self.ReceiveTick`
  (params (DeltaSeconds :type "Float (single-precision)"))
  ;[1 1 1] Set Vars
  (set `self.TimeElapsed` (+ DeltaSeconds (`self.TimeElapsed`)))
  (set `self.TimeSinceLastCollision` (+ DeltaSeconds (`self.TimeSinceLastCollision`))))

(fn `UserConstructionScript`)